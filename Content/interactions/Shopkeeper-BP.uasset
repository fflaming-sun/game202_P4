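; Shopkeeper interaction Blueprint that picks a greeting based on the player character's stats when an actor begins overlapping it.
; On overlap it flags PlayerOverlapping, reads the player's Charisma and Compassion, and sets InterText to a wary, friendly or warm line, the latter two pointing to the jukebox.
; It then calls the parent overlap logic, which is skipped when no stat branch matches.
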(event `self.ReceiveActorBeginOverlap`
  (params (OtherActor :type "Actor Object Reference"))
  (set `self.PlayerOverlapping` true)
  (bind _asbp_third_person_character (cast `/Game/ThirdPerson/Blueprints/BP_ThirdPersonCharacter` (`GameplayStatics.GetPlayerCharacter` 0)))
  (bind _charisma (`/Game/ThirdPerson/Blueprints/BP_ThirdPersonCharacter.Charisma` _asbp_third_person_character))
  (if (< _charisma 0)
    (set `self.InterText` "\"Hey pipsqueak. I've seen you around here before. No funny business here, yea?\"")
    (`parent.ReceiveActorBeginOverlap` OtherActor :!label _label)
    (else
      (bind _returnvalue (> _charisma 5))
      (bind _compassion (`/Game/ThirdPerson/Blueprints/BP_ThirdPersonCharacter.Compassion` _asbp_third_person_character))
      (if (and _returnvalue (<= _compassion 0))
        (set `self.InterText` "\"Hey. What can I get for ya? Make sure to have a look at the jukebox. Authentic 1940s!\"")
        (goto _label)
        (elif (and _returnvalue (>= _compassion 5))
          (set `self.InterText` "\"Hello there! Someone just bought this in, you look like you'd enjoy this! Check it out on the jukebox.\"")
          (goto _label))))))

(event `self.ReceiveTick`
  (params (DeltaSeconds :type "Float (single-precision)"))
  (`parent.ReceiveTick` DeltaSeconds))

(fn `UserConstructionScript`
  (`parent.UserConstructionScript`))